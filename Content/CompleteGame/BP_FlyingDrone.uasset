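; Flying drone actor that calls MoveToNextPoint on the third-person character entering its sphere, gated by tutorial and level progress.
; With TutorialDone set, it passes NewLocation in an immediate call, then repeats the call for each completed level flag (1 to 3) on the player character.
; Without TutorialDone, only the Level 1 flag is checked.
; Tick and construction script are empty.
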(event `self.ReceiveBeginPlay`)

(event `self.Sphere.OnComponentBeginOverlap`
  (params (OverlappedComponent :type "PrimitiveComponent Object Reference") (OtherActor :type "Actor Object Reference") (OtherComp :type "PrimitiveComponent Object Reference") (OtherBodyIndex :type Integer) (bFromSweep :type Boolean) (SweepResult :type "HitResult Structure (by ref)"))
  (bind (_asbp_third_person_character _bsuccess) (cast `/Game/CompleteGame/BP_ThirdPersonCharacter` (`GameplayStatics.GetPlayerCharacter` 0) :!pure true))
  (if (`self.TutorialDone`)
    (bind _asbp_third_person_character_2 (cast `/Game/CompleteGame/BP_ThirdPersonCharacter` OtherActor))
    (`/Game/CompleteGame/BP_ThirdPersonCharacter.MoveToNextPoint` _asbp_third_person_character_2 (`self.NewLocation`))
    (if _bsuccess
      (`|ExecutionSequence`
        (:`then_0`
          (if (`/Game/CompleteGame/BP_ThirdPersonCharacter.IsLevel1Done` _asbp_third_person_character) :!label _label
            (bind _asbp_third_person_character_3 (cast `/Game/CompleteGame/BP_ThirdPersonCharacter` OtherActor))
            (`/Game/CompleteGame/BP_ThirdPersonCharacter.MoveToNextPoint` _asbp_third_person_character_3 (`self.NewLocation`))))
        (:`then_1`
          (if (`/Game/CompleteGame/BP_ThirdPersonCharacter.IsLevel2Done` _asbp_third_person_character)
            (bind _asbp_third_person_character_4 (cast `/Game/CompleteGame/BP_ThirdPersonCharacter` OtherActor))
            (`/Game/CompleteGame/BP_ThirdPersonCharacter.MoveToNextPoint` _asbp_third_person_character_4 (`self.NewLocation`))))
        (:`then_2`
          (if (`/Game/CompleteGame/BP_ThirdPersonCharacter.IsLevel3Done` _asbp_third_person_character)
            (bind _asbp_third_person_character_5 (cast `/Game/CompleteGame/BP_ThirdPersonCharacter` OtherActor))
            (`/Game/CompleteGame/BP_ThirdPersonCharacter.MoveToNextPoint` _asbp_third_person_character_5 (`self.NewLocation`))))))
    (else
      (goto _label))))

(fn `UserConstructionScript`)