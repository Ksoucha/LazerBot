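; BP_DestroyBarriers is a helper actor that removes four referenced barriers from the level when triggered.
; On BeginPlay it registers itself on the player's BP_ThirdPersonCharacter, giving the character a reference to it.
; Its DestroyBarriers function destroys the First through Fourth actors, then starts the same warp sound through both SpawnSound2D and PlaySound2D.
; The call to that function lies outside this Blueprint.
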(event `self.ReceiveBeginPlay`
  (bind _asbp_third_person_character (cast `/Game/CompleteGame/BP_ThirdPersonCharacter` (`GameplayStatics.GetPlayerCharacter` 0)))
  (set `/Game/CompleteGame/BP_ThirdPersonCharacter.DestroyBarriers` self _asbp_third_person_character))

(fn `DestroyBarriers`
  (`self.K2_DestroyActor` (`self.First`))
  (`self.K2_DestroyActor` (`self.Second`))
  (`self.K2_DestroyActor` (`self.Third`))
  (`self.K2_DestroyActor` (`self.Fourth`))
  (`GameplayStatics.SpawnSound2D` "/Game/CompleteGame/Music/warp-306033.warp-306033" 1.0 1.0 0.0 null)
  (`GameplayStatics.PlaySound2D` "/Game/CompleteGame/Music/warp-306033.warp-306033" 1.0 1.0 0.0 null null))

(fn `UserConstructionScript`)