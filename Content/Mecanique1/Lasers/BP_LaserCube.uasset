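; BP_LaserCube is a puzzle-style cube that re-emits a laser when one hits it.
; LaserBounce spawns a BP_Laser at the Arrow, its Z axis along the arrow's forward, inheriting color and spawn reference, with a "C"-updated ID.
; The new laser attaches to SMParent and registers in LasersAttached and the source's ChildLasers.
; A false hit response instead tells the source to clear all attached lasers.
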(fn `LaserBounce`
  (params (LaserHit :type "/Game/Mecanique1/Lasers/BP_Laser Object Reference") (HitResponse :type Boolean) (HitInfo :type "HitResult Structure"))
  (returns (NewLaser :type "/Game/Mecanique1/Lasers/BP_Laser Object Reference"))
  (bind _laserhit (`local.LaserHit`))
  (`/Engine/EditorBlueprintResources/StandardMacros.IsValid` LaserHit
    (:`Is Valid`
      (bind _output_get (set `self.SpawnReference` (`/Game/Mecanique1/Lasers/BP_LaserParent.SpawnReference` LaserHit)))
      (bind _output_get_2 (set `self.Active` HitResponse))
      (`KismetSystemLibrary.PrintString` (`KismetStringLibrary.Conv_BoolToString` _output_get_2))
      (if _output_get_2
        ;[1 1 1] Spawn a new laser if the LaserCube was hit by a laser
        (bind _returnvalue (`|SpawnActorFromClass` "/Game/Mecanique1/Lasers/BP_Laser.BP_Laser_C" (`KismetMathLibrary.MakeTransform` (`SceneComponent.K2_GetComponentLocation` (`self.Arrow`)) (`KismetMathLibrary.MakeRotFromZ` (`SceneComponent.GetForwardVector` (`self.Arrow`)))) "Undefined" "MultiplyWithRoot" null (`/Game/Mecanique1/Lasers/BP_Laser.UpdateID` _laserhit "C") (`/Game/Mecanique1/Lasers/BP_LaserParent.LaserColor` _laserhit) (`self.SpawnReference`) null))
        (set `self.Active` (not HitResponse))
        (`self.K2_AttachToComponent` _returnvalue (`self.SM_Parent`) "None" "KeepWorld" "KeepWorld" "KeepRelative" false)
        (`KismetArrayLibrary.Array_Add` (`self.LasersAttached`) _returnvalue)
        (`KismetArrayLibrary.Array_Add` (`/Game/Mecanique1/Lasers/BP_LaserSpawn.ChildLasers` (`self.SpawnReference`)) _returnvalue)
        (return _returnvalue)
        (else
          (`self.ClearAllLasersAttached` _output_get))))))

(fn `UserConstructionScript`
  (`parent.UserConstructionScript`))