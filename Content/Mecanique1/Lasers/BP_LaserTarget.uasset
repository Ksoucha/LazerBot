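; BP_LaserTarget is a target that changes color when lasers hit it and awards score to the player character.
; LaserBounce stores the hit response as Active and passes the laser's color to TargetHit, which tints a dynamic material.
; A HitColor array tracks incoming colors, restoring the last remaining one when a laser leaves.
; A ScoreAdded flag prevents repeat scoring, and score is removed once one or fewer colors remain.
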(fn `LaserBounce`
  (params (LaserHit :type "/Game/Mecanique1/Lasers/BP_Laser Object Reference") (HitResponse :type Boolean) (HitInfo :type "HitResult Structure"))
  (returns (NewLaser :type "/Game/Mecanique1/Lasers/BP_Laser Object Reference"))
  (set `self.Active` HitResponse)
  (`self.TargetHit` (`/Game/Mecanique1/Lasers/BP_LaserParent.LaserColor` LaserHit))
  (return null))

(fn `TargetHit`
  (params (Color :type "LinearColor Structure"))
  (bind _hitcolor (`self.HitColor`))
  (bind _active (`self.Active`))
  (bind _hitcolor_2 (`self.HitColor`))
  (bind _hitcolor_3 (`self.HitColor`))
  (bind _returnvalue (`PrimitiveComponent.CreateDynamicMaterialInstance` (`self.SM_Parent`) 0 "/Game/LevelPrototyping/Materials/M_Solid.M_Solid" "None"))
  (`MaterialInstanceDynamic.SetVectorParameterValue` _returnvalue "Base Color" (`KismetMathLibrary.SelectColor` Color (`|GetArrayItem` _hitcolor_2 (- (`KismetArrayLibrary.Array_Length` _hitcolor_2) 1)) _active))
  (bind _asbp_third_person_character (cast `/Game/ThirdPerson/Blueprints/BP_ThirdPersonCharacter` (`GameplayStatics.GetPlayerCharacter` 0)))
  (if _active
    (`KismetArrayLibrary.Array_Add` (`self.HitColor`) Color)
    (if (not (`self.ScoreAdded`))
      (`/Game/ThirdPerson/Blueprints/BP_ThirdPersonCharacter.AddScore` _asbp_third_person_character)
      (set `self.ScoreAdded` true))
    (else
      (`KismetArrayLibrary.Array_RemoveItem` _hitcolor_3 Color)
      (`MaterialInstanceDynamic.SetVectorParameterValue` _returnvalue "Base Color" (`|GetArrayItem` _hitcolor (- (`KismetArrayLibrary.Array_Length` _hitcolor) 1)))
      (if (<= (`KismetArrayLibrary.Array_Length` _hitcolor_3) 1)
        (`/Game/ThirdPerson/Blueprints/BP_ThirdPersonCharacter.RemoveScore` _asbp_third_person_character)
        (set `self.ScoreAdded` false)))))

(fn `UserConstructionScript`
  (`parent.UserConstructionScript`))