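; BP_LaserReflect is a reflective object that bounces lasers hitting it by spawning child BP_Laser actors.
; On a hit, LaserBounce spawns a laser at the impact point, mirrored about the surface normal, inheriting color and spawn reference with an updated ID.
; The new laser registers both locally and in the spawn reference's child lasers.
; When the hit ends, attached lasers whose IDs contain the incoming laser's ID are destroyed.
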(fn `CalculateRotation`
  (params (ImpactPoint :type "Vector Structure") (ImpactNormal :type "Vector Structure") (TraceStart :type "Vector Structure"))
  (returns (ReturnValue :type "Rotator Structure"))
  (return (`KismetMathLibrary.MakeRotFromZ` (`KismetMathLibrary.MirrorVectorByNormal` (- ImpactPoint TraceStart) ImpactNormal))))

(fn `ClearAttachedLasers`
  (params (ID_Clear :type String))
  (bind (_arrayindex _arrayelement) (`/Engine/EditorBlueprintResources/StandardMacros.ReverseForEachLoop` (`self.LasersAttached`))
    (:`LoopBody`
      (`/Engine/EditorBlueprintResources/StandardMacros.IsValid` _arrayelement
        (:`Is Valid`
          (if (`KismetStringLibrary.Contains` (`/Game/Mecanique1/Lasers/BP_Laser.LaserID` _arrayelement) (`local.ID_Clear`))
            (`self.K2_DestroyActor` _arrayelement)
            (`KismetArrayLibrary.Array_RemoveItem` (`self.LasersAttached`) _arrayelement)))))))

(fn `LaserBounce`
  (params (LaserHit :type "/Game/Mecanique1/Lasers/BP_Laser Object Reference") (HitResponse :type Boolean) (HitInfo :type "HitResult Structure"))
  (returns (NewLaser :type "/Game/Mecanique1/Lasers/BP_Laser Object Reference"))
  (bind _laserhit (`local.LaserHit`))
  (bind (_bblockinghit _binitialoverlap _time _distance _location _impactpoint _normal _impactnormal _physmat _hitactor _hitcomponent _hitbonename _bonename _hititem _elementindex _faceindex _tracestart) (`GameplayStatics.BreakHitResult` (`local.HitInfo`)))
  (if HitResponse
    ;[1 1 1] Spawn new lasers if the laser hit a LaserReflect object
    (bind _returnvalue (`|SpawnActorFromClass` "/Game/Mecanique1/Lasers/BP_Laser.BP_Laser_C" (`KismetMathLibrary.MakeTransform` _impactpoint (`self.CalculateRotation` _impactpoint _impactnormal _tracestart)) "Undefined" "MultiplyWithRoot" null (`/Game/Mecanique1/Lasers/BP_Laser.UpdateID` _laserhit "B") (`/Game/Mecanique1/Lasers/BP_LaserParent.LaserColor` _laserhit) (`/Game/Mecanique1/Lasers/BP_LaserParent.SpawnReference` _laserhit) null))
    (`KismetArrayLibrary.Array_Add` (`self.LasersAttached`) _returnvalue)
    (`KismetArrayLibrary.Array_Add` (`/Game/Mecanique1/Lasers/BP_LaserSpawn.ChildLasers` (`/Game/Mecanique1/Lasers/BP_LaserParent.SpawnReference` (`local.LaserHit`))) _returnvalue)
    (return _returnvalue)
    (else
      (`self.ClearAttachedLasers` (`/Game/Mecanique1/Lasers/BP_Laser.LaserID` (`local.LaserHit`))))))

(fn `UserConstructionScript`
  (`parent.UserConstructionScript`))