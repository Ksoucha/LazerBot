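; BP_Laser is a colored laser beam that can bounce off objects implementing BPI_Lasers.
; Each tick it box-traces along its up vector, scales its mesh to the hit distance and messages new hit actors to obtain a bounce laser.
; On an unchanged BP_LaserReflect hit it repositions and rotates that bounce laser; on a target change SpawnReference removes following lasers.
; CancelTargetHit releases or deactivates the last target, destroying the laser unless overridden.
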(event `self.ReceiveBeginPlay`
  (`self.ChangeColor`))

(event `self.ReceiveTick`
  (params (DeltaSeconds :type "Float (single-precision)"))
  (`self.SetEndPoint`))

(fn `CancelTargetHit`
  (params (Override :type Boolean))
  (returns (RemoveFromArray :type Boolean))
  (`|ExecutionSequence`
    (:`then_0`
      (bind _lasthitactor (`self.LastHitActor`)
        (:`then`
          (bind _asbp_laser_parent (cast `/Game/Mecanique1/Lasers/BP_LaserParent` _lasthitactor))
          (if (and (`KismetSystemLibrary.DoesImplementInterface` _asbp_laser_parent "/Game/Mecanique1/Lasers/BPI_Lasers.BPI_Lasers_C") (`KismetArrayLibrary.Array_IsEmpty` (`/Game/Mecanique1/Lasers/BP_LaserParent.LasersAttached` _asbp_laser_parent)))
            (message `/Game/Mecanique1/Lasers/BPI_Lasers.LaserBounce` (`self.LastHitActor`) self false (struct))
            (else
              (set `/Game/Mecanique1/Lasers/BP_LaserParent.Active` false _asbp_laser_parent))))
        (:`else`)))
    (:`then_1`
      (if (`local.Override`)
        (return false)
        (else
          (`self.K2_DestroyActor`)
          (return true))))))

(fn `ChangeColor`
  (bind _returnvalue (`PrimitiveComponent.CreateDynamicMaterialInstance` (`self.SM_Parent`) 0 "/Game/Mecanique1/Lasers/M_Laser.M_Laser" "None"))
  (`MaterialInstanceDynamic.SetVectorParameterValue` _returnvalue "Color" (`self.LaserColor`)))

(fn `SetEndPoint`
  (locals (LaserRange :type "Float (double-precision)" :default 3000.0) (LaserHitInfo :type "HitResult Structure") (LaserHitActor :type "Actor Object Reference"))
  (bind _returnvalue (`self.GetActorUpVector`))
  (bind (_bblockinghit _binitialoverlap _time _distance _location _impactpoint _normal _impactnormal _physmat _hitactor _hitcomponent _hitbonename _bonename _hititem _elementindex _faceindex _tracestart) (`GameplayStatics.BreakHitResult` (`local.LaserHitInfo`)))
  (bind _returnvalue_2 (+ (`self.K2_GetActorLocation`) (* _returnvalue 2.0)))
  ;[1 1 1] Create laser
  (bind _outhit (`KismetSystemLibrary.BoxTraceSingle` _returnvalue_2 (+ _returnvalue_2 (* _returnvalue (`local.LaserRange`))) (0.5 0.5 0.5) (struct) "TraceTypeQuery1"))
  (bind _output_get (set `local.LaserHitInfo` _outhit))
  (bind (_bblockinghit_2 _binitialoverlap_2 _time_2 _distance_2 _location_2 _impactpoint_2 _normal_2 _impactnormal_2 _physmat_2 _hitactor_2) (`GameplayStatics.BreakHitResult` _output_get))
  (set `local.LaserHitActor` _hitactor_2)
  (`SceneComponent.SetWorldScale3D` (`self.SM_Parent`) (`KismetMathLibrary.MakeVector` 0.05 0.05 (`KismetMathLibrary.SelectFloat` (/ (+ _distance_2 1.0) 100.0) (/ (`local.LaserRange`) 100.0) _bblockinghit_2)))
  (`local.LaserHitActor`
    (:`then`
      ;[1 1 1] Check whether the laser is blocked by an object
      (`|ExecutionSequence`
        (:`then_0`
          (if (== (`self.LastHitActor`) (`local.LaserHitActor`))
            (bind _asbp_laser_reflect (cast `/Game/Mecanique1/Lasers/BP_LaserReflect` (`self.LastHitActor`)))
            (`self.K2_SetActorLocation` (`self.BounceLaser`) (`.ImpactPoint` (`GameplayStatics.BreakHitResult` (`local.LaserHitInfo`))) false false)
            (`self.K2_SetActorRotation` (`self.BounceLaser`) (`/Game/Mecanique1/Lasers/BP_LaserReflect.CalculateRotation` _asbp_laser_reflect _impactpoint _impactnormal _tracestart) false)
            (else
              (`|ExecutionSequence`
                (:`then_0`
                  ;[1 1 1] Remove following lasers
                  (if (`KismetSystemLibrary.DoesImplementInterface` (`self.LastHitActor`) "/Game/Mecanique1/Lasers/BPI_Lasers.BPI_Lasers_C")
                    (`/Game/Mecanique1/Lasers/BP_LaserSpawn.RemoveFollowingLasers` (`self.SpawnReference`) self)))
                (:`then_1`
                  ;[1 1 1] Call the function to reflect the laser (BP_LaserReflect)
                  (if (`KismetSystemLibrary.DoesImplementInterface` (`local.LaserHitActor`) "/Game/Mecanique1/Lasers/BPI_Lasers.BPI_Lasers_C")
                    (`self.BounceLaser`
                      (:`then`)
                      (:`else`
                        (bind _newlaser (message `/Game/Mecanique1/Lasers/BPI_Lasers.LaserBounce` (`local.LaserHitActor`) self true (`local.LaserHitInfo`)))
                        (set `self.BounceLaser` _newlaser)))))))))
        (:`then_1`
          (set `self.LastHitActor` (`local.LaserHitActor`)))))
    (:`else`
      (if (`KismetSystemLibrary.DoesImplementInterface` (`local.LaserHitActor`) "/Game/Mecanique1/Lasers/BPI_Lasers.BPI_Lasers_C")
        (`self.BounceLaser`
          (:`then`)
          (:`else`
            (bind _newlaser_2 (message `/Game/Mecanique1/Lasers/BPI_Lasers.LaserBounce` (`local.LaserHitActor`) self true (`local.LaserHitInfo`)))
            (set `self.BounceLaser` _newlaser_2)
            (set `self.LastHitActor` (`local.LaserHitActor`))))
        (else
          (set `self.LastHitActor` (`local.LaserHitActor`)))))))

(fn `UpdateID`
  (params (Append :type String))
  (returns (ReturnValue :type String))
  (return (`KismetStringLibrary.Concat_StrStr` (`self.LaserID`) Append)))

(fn `UserConstructionScript`
  (`parent.UserConstructionScript`))