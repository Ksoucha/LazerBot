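; Laser emitter that spawns a BP_Laser at its arrow on BeginPlay, passing its color, a self reference and its display name as the laser ID.
; It tracks lasers in ChildLasers, starting with that first one.
; RemoveFollowingLasers walks the list in reverse, calls CancelTargetHit on lasers whose ID contains the given laser's ID, flagging exact matches, and drops those returning true.
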(event `self.ReceiveBeginPlay`
  (set `self.SpawnReference` self)
  (set `self.ID` (`KismetSystemLibrary.GetDisplayName` self))
  (bind _returnvalue (`|SpawnActorFromClass` "/Game/Mecanique1/Lasers/BP_Laser.BP_Laser_C" (`KismetMathLibrary.MakeTransform` (`SceneComponent.K2_GetComponentLocation` (`self.Arrow`)) (`self.K2_GetActorRotation`)) "Undefined" "MultiplyWithRoot" null (`self.ID`) (`self.LaserColor`) (`self.SpawnReference`) null))
  (`KismetArrayLibrary.Array_Add` (`self.ChildLasers`) _returnvalue))

(fn `RemoveFollowingLasers`
  (params (LaserReference :type "/Game/Mecanique1/Lasers/BP_Laser Object Reference"))
  (locals (LaserIDRemoved :type String))
  (set `local.LaserIDRemoved` (`/Game/Mecanique1/Lasers/BP_Laser.LaserID` LaserReference))
  (bind (_arrayindex _arrayelement) (`/Engine/EditorBlueprintResources/StandardMacros.ReverseForEachLoop` (`self.ChildLasers`))
    (:`LoopBody`
      (`/Engine/EditorBlueprintResources/StandardMacros.IsValid` _arrayelement
        (:`Is Valid`
          (if (`KismetStringLibrary.Contains` (`/Game/Mecanique1/Lasers/BP_Laser.LaserID` _arrayelement) (`local.LaserIDRemoved`))
            (bind _removefromarray (`/Game/Mecanique1/Lasers/BP_Laser.CancelTargetHit` _arrayelement (`KismetStringLibrary.EqualEqual_StrStr` (`/Game/Mecanique1/Lasers/BP_Laser.LaserID` _arrayelement) (`local.LaserIDRemoved`))))
            (if _removefromarray
              (`KismetArrayLibrary.Array_RemoveItem` (`self.ChildLasers`) _arrayelement))))))))

(fn `UserConstructionScript`
  (`parent.UserConstructionScript`))